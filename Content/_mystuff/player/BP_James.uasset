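; BP_James is a player character that carries an AK47, spawned on BeginPlay and attached to a mesh socket.
; Firing plays muzzle flash and sound, then uses two traces: camera forward finds the aim point, and muzzle to that point finds the hit.
; The hit actor takes the rifle's damage with an impact effect, while debug lines and a component-name print remain active.
; Die plays a headshot death montage.
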(event `self.ReceiveBeginPlay`
  (bind _mesh (`self.Mesh`))
  (`parent.ReceiveBeginPlay`)
  (bind _returnvalue (`|SpawnActorFromClass` "/Game/_mystuff/weapons/BP_AK47.BP_AK47_C" (`SceneComponent.GetSocketTransform` _mesh (`self.RifleSocketName`) "RTS_World") "Undefined" "MultiplyWithRoot" null null))
  (bind _output_get (set `self.Rifle` _returnvalue))
  (`self.K2_AttachToComponent` _output_get _mesh "None" "SnapToTarget" "SnapToTarget" "SnapToTarget" true))

(event `EnhancedInput|/Game/_mystuff/Input/Actions/IA_Fire`
  (params (ActionValue :type Boolean) (ElapsedSeconds :type "Float (double-precision)") (TriggeredSeconds :type "Float (double-precision)") (InputAction :type "InputAction Object Reference" :default "/Game/_mystuff/Input/Actions/IA_Fire.IA_Fire"))
  (bind _returnvalue (`GameplayStatics.GetPlayerCameraManager` 0))
  (bind _returnvalue_2 (`self.K2_GetActorLocation` _returnvalue))
  ;[1 1 1] Shoot
  (:`Started`
    (`GameplayStatics.SpawnEmitterAttached` "/Game/InfinityBladeEffects/Effects/FX_Monsters/FX_Monster_Gruntling/Master/P_BackPack_MuzzleFlash.P_BackPack_MuzzleFlash" (`Actor.RootComponent` (`self.Rifle`)) "Muzzle" (0.0 0.0 0.0) (struct) (0.1 0.1 0.1) "KeepWorldPosition")
    (`GameplayStatics.PlaySoundAtLocation` "/Game/_mystuff/MS_RifleFire.MS_RifleFire" (`self.K2_GetActorLocation`) (struct) 0.3 1.0 0.0 null null null null)
    (bind _outhit (`KismetSystemLibrary.LineTraceSingle` :`Start` _returnvalue_2 :`End` (+ _returnvalue_2 (* (`self.GetActorForwardVector` _returnvalue) 10000.0)) :`TraceChannel` "TraceTypeQuery1" :`DrawDebugType` "ForDuration" :`bIgnoreSelf` false))
    (bind (_bblockinghit _binitialoverlap _time _distance _location _impactpoint _normal _impactnormal _physmat _hitactor _hitcomponent _hitbonename _bonename _hititem _elementindex _faceindex _tracestart _traceend) (`GameplayStatics.BreakHitResult` _outhit))
    (bind _outhit_2 (`KismetSystemLibrary.LineTraceSingle` :`Start` (`SceneComponent.GetSocketLocation` (`/Game/_mystuff/weapons/BP_AK47.AK47` (`self.Rifle`)) "Muzzle") :`End` (select `bool` (!= _impactpoint (0.0 0.0 0.0)) :`false` _traceend :`true` _impactpoint) :`TraceChannel` "TraceTypeQuery1" :`DrawDebugType` "ForDuration" :`bIgnoreSelf` false))
    (bind (_bblockinghit_2 _binitialoverlap_2 _time_2 _distance_2 _location_2 _impactpoint_2 _normal_2 _impactnormal_2 _physmat_2 _hitactor_2 _hitcomponent_2) (`GameplayStatics.BreakHitResult` _outhit_2))
    (`KismetSystemLibrary.PrintString` (`KismetSystemLibrary.GetDisplayName` _hitcomponent_2))
    (`GameplayStatics.ApplyDamage` _hitactor_2 (`/Game/_mystuff/weapons/BP_AK47.Damage` (`self.Rifle`)))
    (`GameplayStatics.SpawnEmitterAtLocation` "/Game/InfinityBladeEffects/Effects/FX_Monsters/FX_Monster_Troll/death/P_TrollDeathImpact.P_TrollDeathImpact" _impactpoint_2 (`KismetMathLibrary.MakeRotFromX` _normal_2) (0.5 0.5 0.5))))

(fn `Die`
  (`self.PlayAnimMontage` "/Game/_mystuff/player/james/animations/rifle/AM_death_from_front_headshot.AM_death_from_front_headshot"))

(fn `UserConstructionScript`
  (`parent.UserConstructionScript`))