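; Enemy character Blueprint, named as a backup, with health, a camera-facing health bar, a melee attack and a death animation.
; Tick updates the WBP_EnemyHealth widget from Health and turns it toward the camera.
; Attack sphere-traces for pawns along a zero-rotation forward vector, then plays a swipe montage and damages a hit BP_ThirdPersonCharacter.
; AnyDamage reduces Health and calls Die at zero, which only plays the dying montage.
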(event `self.ReceiveTick`
  (params (DeltaSeconds :type "Float (single-precision)"))
  ;[1 1 1] Health
  (bind _aswbp_enemy_health (cast `/Game/_mystuff/enemy/WBP_EnemyHealth` (`WidgetComponent.GetWidget` (`self.Health Bar`))))
  (`ProgressBar.SetPercent` (`/Game/_mystuff/enemy/WBP_EnemyHealth.HealthBar` _aswbp_enemy_health) (/ (`self.Health`) 100.0))
  (`SceneComponent.K2_SetWorldRotation` (`self.Health Bar`) (`KismetMathLibrary.FindLookAtRotation` (`self.K2_GetActorLocation`) (`self.K2_GetActorLocation` (`GameplayStatics.GetPlayerCameraManager` 0))) false false))

(event `Attack`
  (bind _returnvalue (`self.K2_GetActorLocation`))
  ;[1 1 1] Attack
  (bind (_outhit _returnvalue_2) (`KismetSystemLibrary.SphereTraceSingleForObjects` :`Start` _returnvalue :`End` (+ _returnvalue (* (`KismetMathLibrary.GetForwardVector` (struct)) 250.0)) :`Radius` 120.0 :`ObjectTypes` (`|MakeArray` "ObjectTypeQuery3" :!type "EObjectTypeQuery Enum") :`DrawDebugType` "ForDuration"))
  (if _returnvalue_2
    (bind (_bblockinghit _binitialoverlap _time _distance _location _impactpoint _normal _impactnormal _physmat _hitactor) (`GameplayStatics.BreakHitResult` _outhit))
    (cast `/Game/_mystuff/player/BP_ThirdPersonCharacter` _hitactor)
    (`KismetSystemLibrary.PrintString` "Attacking")
    (`self.PlayAnimMontage` "/Game/_mystuff/enemy/creature/animations/AM_MutantSwipe.AM_MutantSwipe")
    (`GameplayStatics.ApplyDamage` _hitactor (`self.Damage`))))

(event `self.ReceiveAnyDamage`
  (params (Damage :type "Float (single-precision)") (DamageType :type "DamageType Object Reference") (InstigatedBy :type "Controller Object Reference") (DamageCauser :type "Actor Object Reference"))
  ;[1 1 1] Take Damage
  (`KismetSystemLibrary.PrintString` "Enemy Took Damage")
  (set `self.Health` (- (`self.Health`) Damage))
  (if (<= (`self.Health`) 0.0)
    (`self.Die`)))

(fn `Die`
  (`self.PlayAnimMontage` "/Game/_mystuff/enemy/creature/animations/AM_mutant_dying.AM_mutant_dying"))

(fn `UserConstructionScript`)